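; Generic enemy character with clamped health that is destroyed when damage brings it to zero.
; Tick pushes current health into the enemy's health bar widget and, while IsHit is set, adds slight forward movement.
; Capsule overlap sets IsHit when the other actor is a BP_IcePick and clears it on end overlap.
; An Attack function, not called within this Blueprint, plays a cast montage and spawns a flame ball at CastArrow.
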(event OnComponentBeginOverlap(CapsuleComponent)
  (params (OverlappedComponent :type Primitive%20Component%20Object%20Reference) (OtherActor :type Actor%20Object%20Reference) (OtherComp :type Primitive%20Component%20Object%20Reference) (OtherBodyIndex :type Integer) (bFromSweep :type Boolean) (SweepResult :type Hit%20Result%20Structure%20%28by%20ref%29))
  (Variables|Default|SetisHit (== (Utilities|GetClass OtherActor) "/Game/projectiles/BP_IcePick.BP_IcePick_C"))
  (Development|PrintString "Hit"))

(event OnComponentEndOverlap(CapsuleComponent)
  (params (OverlappedComponent :type Primitive%20Component%20Object%20Reference) (OtherActor :type Actor%20Object%20Reference) (OtherComp :type Primitive%20Component%20Object%20Reference) (OtherBodyIndex :type Integer))
  (Variables|Default|SetisHit false))

(event OnComponentHit(CapsuleComponent)
  (params (HitComponent :type Primitive%20Component%20Object%20Reference) (OtherActor :type Actor%20Object%20Reference) (OtherComp :type Primitive%20Component%20Object%20Reference) (NormalImpulse :type Vector :default "0, 0, 0") (Hit :type Hit%20Result%20Structure%20%28by%20ref%29)))

(event EventBeginPlay)

(event Collision|EventActorBeginOverlap
  (params (OtherActor :type Actor%20Object%20Reference)))

(event EventTick
  (params (DeltaSeconds :type Float%20%28single-precision%29))
  (Utilities|FlowControl|Sequence
    (:then_0
      (CallFunction|UpdateHealthBar))
    (:then_1
      (if (Variables|Default|GetisHit)
        (Pawn|Input|AddMovementInput (Math|Vector|GetForwardVector (Variables|/Script/Engine.MovementComponent|GetUpdatedPrimitive (Variables|Character|GetCharacterMovement))) 0.1 false)))))

(event Game|Damage|EventAnyDamage
  (params (Damage :type Float%20%28single-precision%29) (DamageType :type Damage%20Type%20Object%20Reference) (InstigatedBy :type Controller%20Object%20Reference) (DamageCauser :type Actor%20Object%20Reference))
  (bind _output_get (Variables|Default|Sethealth (Math|Float|Clamp(Float) (- (Variables|Default|Gethealth) Damage) 0.0 1e+02)))
  (Development|PrintString (Utilities|String|ToString(Float) Damage))
  (if (<= _output_get 0.0)
    (Actor|DestroyActor)))

(fn ConstructionScript)

(fn UpdateHealthBar
  (bind _asenemy_helath_bar (Utilities|Casting|CastToEnemyHelathBar (UserInterface|GetUserWidgetObject (Variables|Default|GetEnemyHelth))))
  (Variables|/Game/UI/EnemyHelathBar.EnemyHelathBar_C|SetEnemyHealth _asenemy_helath_bar (Variables|Default|Gethealth))
  (return))

(fn Attack
  (bind _returnvalue (Animation|PlayAnimMontage "/Game/GameModes/ThirdPerson/Characters/Mannequins/Animations/Manny/M_IdleCast.M_IdleCast" 0.5 "None"))
  (Game|SpawnActorfromClass "/Game/projectiles/BP_FlameBall.BP_FlameBall_C" (Transformation|GetWorldTransform (Variables|Default|GetCast%20Arrow)) "AlwaysSpawn" "MultiplyWithRoot" 0 0)
  (Development|PrintString (Utilities|String|ToString(Float) _returnvalue))
  (return _returnvalue))