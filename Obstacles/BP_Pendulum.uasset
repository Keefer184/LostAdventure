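; BP_Pendulum is a swinging obstacle that applies point damage to any actor its Ball1 component hits.
; OnActivate starts a timeline that drives the pitch of the Joint component.
; A three-second Delay on that timeline's update starts a second timeline in reverse on the same pitch.
; That timeline's update uses another Delay before StartOver replays the first, looping the swing.
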(event OnComponentHit(Ball1)
  (params (HitComponent :type Primitive%20Component%20Object%20Reference) (OtherActor :type Actor%20Object%20Reference) (OtherComp :type Primitive%20Component%20Object%20Reference) (NormalImpulse :type Vector :default "0, 0, 0") (Hit :type Hit%20Result%20Structure%20%28by%20ref%29))
  (Game|Damage|ApplyPointDamage OtherActor 1.0 NormalImpulse Hit))

(event Custom|StartOver
  (bind _newtrack_0 (Timeline|Timeline PlayFromStart)
    (:Update
      (Transformation|SetRelativeRotation (Variables|Default|GetJoint) (Math|Rotator|MakeRotator 0.0 _newtrack_0 0.0) false false)
      (Utilities|FlowControl|Delay 3.0)
      (bind _newtrack_0_2 (Timeline|Timeline_0 ReverseFromEnd)
        (:Update
          (Transformation|SetRelativeRotation (Variables|Default|GetJoint) (Math|Rotator|MakeRotator 0.0 _newtrack_0_2 0.0) false false)
          (Utilities|FlowControl|Delay 3.0)
          (CallFunction|StartOver))))))

(event EventOnActivate
  (bind _newtrack_0 (Timeline|Timeline PlayFromStart)
    (:Update
      (Transformation|SetRelativeRotation (Variables|Default|GetJoint) (Math|Rotator|MakeRotator 0.0 _newtrack_0 0.0) false false)
      (Utilities|FlowControl|Delay 3.0)
      (bind _newtrack_0_2 (Timeline|Timeline_0 ReverseFromEnd)
        (:Update
          (Transformation|SetRelativeRotation (Variables|Default|GetJoint) (Math|Rotator|MakeRotator 0.0 _newtrack_0_2 0.0) false false)
          (Utilities|FlowControl|Delay 3.0)
          (CallFunction|StartOver))))))

(fn ConstructionScript)