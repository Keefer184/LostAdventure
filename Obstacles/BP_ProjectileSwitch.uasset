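; BP_ProjectileSwitch is a one-shot trigger switch obstacle that activates a linked arrow trap.
; The first overlap with its Box sets IsTriggered, which blocks any later activation.
; It then lowers the root component slightly in a single step, like a pressed plate, and calls OnActivateMessage on the referenced TriggeredArrows.
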(event OnComponentBeginOverlap(Box)
  (params (OverlappedComponent :type Primitive%20Component%20Object%20Reference) (OtherActor :type Actor%20Object%20Reference) (OtherComp :type Primitive%20Component%20Object%20Reference) (OtherBodyIndex :type Integer) (bFromSweep :type Boolean) (SweepResult :type Hit%20Result%20Structure%20%28by%20ref%29))
  (bind _defaultsceneroot (Variables|Default|GetDefaultSceneRoot))
  (bind _relativelocation (Variables|/Script/Engine.SceneComponent|GetRelativeLocation _defaultsceneroot))
  (if (not (Variables|Default|GetisTriggered))
    (Variables|Default|SetisTriggered true)
    (Utilities|FlowControl|Sequence
      (:then_0
        (Transformation|SetRelativeLocation (Variables|Default|GetDefaultSceneRoot) (Math|Vector|MakeVector (.x _relativelocation) (.y _relativelocation) (- (.z _relativelocation) 5.0)) false false))
      (:then_1
        (Class|BPIElectricity|OnActivate(Message) (Variables|Default|GetTriggeredArrows))))))

(fn ConstructionScript)