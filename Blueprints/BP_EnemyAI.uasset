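; Enemy AI pawn that patrols random reachable points, chases the player on sight and casts flame balls.
; PawnSensing switches it to an AI MoveTo chase loop that spawns BP_FlameBall with a cast montage on arrival, falling back to patrol if the move fails.
; Overlapping BP_IcePick forces forward movement input and reveals the health bar.
; Damage lowers clamped health, destroying it at zero; the health bar widget updates every Tick.
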(event OnSeePawn(PawnSensing)
  (params (Pawn :type Pawn%20Object%20Reference))
  ;[1 1 1] Follow
  (Variables|Default|SetisSeingPlayer true)
  (CallFunction|FollowPlayer)
  (Rendering|SetVisibility (Variables|Default|GetHealthBar) true false))

(event OnComponentBeginOverlap(CapsuleComponent)
  (params (OverlappedComponent :type Primitive%20Component%20Object%20Reference) (OtherActor :type Actor%20Object%20Reference) (OtherComp :type Primitive%20Component%20Object%20Reference) (OtherBodyIndex :type Integer) (bFromSweep :type Boolean) (SweepResult :type Hit%20Result%20Structure%20%28by%20ref%29))
  ;[1 1 1] Damage System
  (Variables|Default|Setishit (== (Utilities|GetClass OtherActor) "/Game/projectiles/BP_IcePick.BP_IcePick_C"))
  (Rendering|SetVisibility (Variables|Default|GetHealthBar) true false))

(event OnComponentEndOverlap(CapsuleComponent)
  (params (OverlappedComponent :type Primitive%20Component%20Object%20Reference) (OtherActor :type Actor%20Object%20Reference) (OtherComp :type Primitive%20Component%20Object%20Reference) (OtherBodyIndex :type Integer))
  ;[1 1 1] Damage System
  (Variables|Default|Setishit false))

(event Custom|Follow%20Player
  ;[1 1 1] Follow commands
  (if (Variables|Default|GetisSeingPlayer)
    (AI|AIMoveTo self "0, 0, 0" (Game|GetPlayerCharacter 0) 5e+02 false :!label _label
      (:OnSuccess
        ;[1 1 1] Attack
        (if (Variables|Default|GetcanAttack)
          (Variables|Default|SetcanAttack false)
          (Game|SpawnActorfromClass "/Game/projectiles/BP_FlameBall.BP_FlameBall_C" (Transformation|GetWorldTransform (Variables|Default|GetCast%20Arrow)) "AlwaysSpawn" "MultiplyWithRoot" 0 0)
          (bind _returnvalue (Animation|PlayAnimMontage "/Game/GameModes/ThirdPerson/Characters/Mannequins/Animations/Manny/MW_IdleCast.MW_IdleCast" 0.5 "None"))
          (Utilities|FlowControl|Delay _returnvalue)
          (Variables|Default|SetcanAttack true)
          (goto _label)))
      (:OnFail
        (CallFunction|Patrol)))
    (else
      (Variables|Default|SetisSeingPlayer false))))

(event Custom|Patrol
  (bind _self self)
  (bind _self_2 self)
  ;[1 1 1] Patrol
  (Rendering|SetVisibility (Variables|Default|GetHealthBar) false false)
  (AI|AIMoveTo _self_2 (.RandomLocation (AI|Navigation|GetRandomReachablePointinRadius (Pawn|GetNavAgentLocation _self_2) 5e+03 0 0)) 0 5.0 false :!label _label
    (:OnSuccess
      (Utilities|FlowControl|Delay 3.0)
      (AI|AIMoveTo _self (.RandomLocation (AI|Navigation|GetRandomReachablePointinRadius (Pawn|GetNavAgentLocation _self) 5e+03 0 0)) 0 5.0 false
        (:OnSuccess
          (goto _label))))))

(event EventBeginPlay
  ;[1 1 1] Start
  (Utilities|FlowControl|Sequence
    (:then_0
      (if (not (Variables|Default|GetisSeingPlayer))
        (CallFunction|Patrol)))
    (:then_1
      (Rendering|SetVisibility (Variables|Default|GetHealthBar) false false))))

(event EventTick
  (params (DeltaSeconds :type Float%20%28single-precision%29))
  ;[1 1 1] Always do
  (Utilities|FlowControl|Sequence
    (:then_1
      (if (Variables|Default|Getishit)
        (Pawn|Input|AddMovementInput (Math|Vector|GetForwardVector (Variables|/Script/Engine.MovementComponent|GetUpdatedPrimitive (Variables|Character|GetCharacterMovement))) 1.0 true)))
    (:then_2
      (CallFunction|UpdateHealthBar))))

(event Game|Damage|EventAnyDamage
  (params (Damage :type Float%20%28single-precision%29) (DamageType :type Damage%20Type%20Object%20Reference) (InstigatedBy :type Controller%20Object%20Reference) (DamageCauser :type Actor%20Object%20Reference))
  ;[1 1 1] Damage System
  (bind _output_get (Variables|Default|SetHealth (Math|Float|Clamp(Float) (- (Variables|Default|GetHealth) Damage) 0.0 1e+02)))
  (if (<= _output_get 0.0)
    (Actor|DestroyActor)))

(fn ConstructionScript)

(fn UpdateHealthBar
  (bind _asenemy_helath_bar (Utilities|Casting|CastToEnemyHelathBar (UserInterface|GetUserWidgetObject (Variables|Default|GetHealthBar))))
  (bind _output_get (Variables|/Game/UI/EnemyHelathBar.EnemyHelathBar_C|SetEnemyHealth _asenemy_helath_bar (Variables|Default|GetHealth)))
  (return _output_get))