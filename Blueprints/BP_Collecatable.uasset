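; BP_Collecatable is a pickup actor that counts toward a collection goal held in BP_ThirdPersonGameMode.
; Any overlap on its Collide component increments the game mode's CollectableCount, refreshes the HUD counter and destroys the pickup, without checking the overlapping actor.
; Once the count reaches a hard-coded threshold of four, it sets HasEnough and reveals the HUD's HasKey widget.
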(event OnComponentBeginOverlap(Collide)
  (params (OverlappedComponent :type Primitive%20Component%20Object%20Reference) (OtherActor :type Actor%20Object%20Reference) (OtherComp :type Primitive%20Component%20Object%20Reference) (OtherBodyIndex :type Integer) (bFromSweep :type Boolean) (SweepResult :type Hit%20Result%20Structure%20%28by%20ref%29))
  (bind _asbp_third_person_game_mode (Utilities|Casting|CastToBP_ThirdPersonGameMode (Game|GetGameMode)))
  (bind _output_get (Variables|/Game/GameModes/ThirdPerson/Blueprints/BP_ThirdPersonGameMode.BP_ThirdPersonGameMode_C|SetcollectableCount _asbp_third_person_game_mode (+ (Variables|/Game/GameModes/ThirdPerson/Blueprints/BP_ThirdPersonGameMode.BP_ThirdPersonGameMode_C|GetcollectableCount _asbp_third_person_game_mode) 1)))
  (Default|UpdateCollectables (Variables|/Game/GameModes/ThirdPerson/Blueprints/BP_ThirdPersonGameMode.BP_ThirdPersonGameMode_C|GetHud_Ref _asbp_third_person_game_mode))
  (if (>= _output_get 4)
    (Variables|/Game/GameModes/ThirdPerson/Blueprints/BP_ThirdPersonGameMode.BP_ThirdPersonGameMode_C|SethasEnough _asbp_third_person_game_mode true)
    (Widget|SetVisibility (Variables|/Game/UI/W_Hud.W_Hud_C|GetHasKey (Variables|/Game/GameModes/ThirdPerson/Blueprints/BP_ThirdPersonGameMode.BP_ThirdPersonGameMode_C|GetHud_Ref _asbp_third_person_game_mode)) "Visible"))
  (Actor|DestroyActor))

(event EventBeginPlay)

(event Collision|EventActorBeginOverlap
  (params (OtherActor :type Actor%20Object%20Reference)))

(event EventTick
  (params (DeltaSeconds :type Float%20%28single-precision%29)))

(fn ConstructionScript)