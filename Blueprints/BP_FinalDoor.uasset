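; BP_FinalDoor is the game's final door, which leads to the win screen once the game mode's HasEnough flag is set.
; Entering the Box trigger either starts a Timeline that raises the Plane or toggles a W_StatuesNeeded widget, which is removed on exit.
; The Timeline's update adds to the Plane's height, then after a delay pauses the game and shows W_WinGame.
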(event OnComponentBeginOverlap(Box)
  (params (OverlappedComponent :type Primitive%20Component%20Object%20Reference) (OtherActor :type Actor%20Object%20Reference) (OtherComp :type Primitive%20Component%20Object%20Reference) (OtherBodyIndex :type Integer) (bFromSweep :type Boolean) (SweepResult :type Hit%20Result%20Structure%20%28by%20ref%29))
  (bind _asbp_third_person_game_mode (Utilities|Casting|CastToBP_ThirdPersonGameMode (Game|GetGameMode)))
  (if (Variables|/Game/GameModes/ThirdPerson/Blueprints/BP_ThirdPersonGameMode.BP_ThirdPersonGameMode_C|GethasEnough _asbp_third_person_game_mode)
    (Input|EnableInput (Game|GetPlayerController 0))
    (CallFunction|OnActivate)
    (else
      (Utilities|IsValid (Variables|Default|GetStatues)
        (:Is%20Valid
          (Utilities|IsValid (Variables|Default|GetStatues)
            (:Is%20Valid
              (Widget|RemovefromParent (Variables|Default|GetStatues))
              (Variables|Default|SetStatues 0))))
        (:Is%20Not%20Valid
          (bind _returnvalue (UserInterface|CreateWidget "/Game/UI/W_StatuesNeeded.W_StatuesNeeded_C"))
          (bind _output_get (Variables|Default|SetStatues _returnvalue))
          (UserInterface|Viewport|AddtoViewport _output_get 0))))))

(event OnComponentEndOverlap(Box)
  (params (OverlappedComponent :type Primitive%20Component%20Object%20Reference) (OtherActor :type Actor%20Object%20Reference) (OtherComp :type Primitive%20Component%20Object%20Reference) (OtherBodyIndex :type Integer))
  (Input|DisableInput (Game|GetPlayerController 0))
  (Utilities|IsValid (Variables|Default|GetStatues)
    (:Is%20Valid
      (Widget|RemovefromParent (Variables|Default|GetStatues))
      (Variables|Default|SetStatues 0))))

(event EventOnActivate
  (bind _plane (Variables|Default|GetPlane))
  (bind _relativelocation (Variables|/Script/Engine.SceneComponent|GetRelativeLocation _plane))
  (bind _newtrack_0 (Timeline|Timeline PlayFromStart)
    (:Update
      (Transformation|SetRelativeLocation (Variables|Default|GetPlane) (Math|Vector|MakeVector (.x _relativelocation) (.y _relativelocation) (+ (.z _relativelocation) _newtrack_0 1.0)) false false)
      (Utilities|FlowControl|Delay 4.5)
      (Game|SetGamePaused true)
      (bind _returnvalue (UserInterface|CreateWidget "/Game/UI/W_WinGame.W_WinGame_C"))
      (UserInterface|Viewport|AddtoViewport _returnvalue 0))))

(fn ConstructionScript)