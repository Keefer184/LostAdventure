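; BP_Elevator is an elevator that moves through a list of MovementPoints, one leg per OnActivate call, and reports itself as not interactable.
; A timeline lerps the root's relative location from its current position toward the indexed point, without sweep.
; On finish, the index advances and wraps to zero, then calls an empty StartOver event, so movement does not chain.
; An IsDown toggle is left unconnected.
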(event Custom|StartOver
  ;[1 1 1] Kept just in case
)

(event EventOnActivate
  (bind _newtrack_0 (Timeline|MovementTimeline PlayFromStart)
    (:Update
      (Transformation|SetRelativeLocation (Variables|Default|GetDefaultSceneRoot) (Math|Vector|Lerp(Vector) (Variables|/Script/Engine.SceneComponent|GetRelativeLocation (Variables|Default|GetDefaultSceneRoot)) (Utilities|Array|Get(acopy) (Variables|Default|GetMovementPoints) (Variables|Default|GetPointIndex)) _newtrack_0) false false))
    (:Finished
      ;[1 1 1] Index control
      (if (>= (Variables|Default|GetPointIndex) (- (Utilities|Array|Length (Variables|Default|GetMovementPoints)) 1))
        (Variables|Default|SetPointIndex 0)
        (else
          (Math|Integer|IncrementInt (Variables|Default|GetPointIndex)
            (:%20%20
              _))))
      (CallFunction|StartOver))))

(fn ConstructionScript)

(fn IsInteractable
  (return false))